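; One-way door actor whose mesh appears once the player character enters its trigger box.
; On BeginPlay the static mesh is dropped far below its placed position and hidden.
; The first player overlap with the Box makes it visible and teleports or snaps it back up, with a DoOnce that is never reset, so the door stays in place.
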(event OnComponentBeginOverlap(Box)
  (params (OverlappedComponent :type Primitive%20Component%20Object%20Reference) (OtherActor :type Actor%20Object%20Reference) (OtherComp :type Primitive%20Component%20Object%20Reference) (OtherBodyIndex :type Integer) (bFromSweep :type Boolean) (SweepResult :type Hit%20Result%20Structure%20%28by%20ref%29))
  (bind _staticmesh (Variables|Default|GetStaticMesh))
  (if (== OtherActor (Game|GetPlayerCharacter 0))
    (Utilities|FlowControl|DoOnce false
      (:Completed
        (Rendering|SetVisibility _staticmesh true false)
        (Transformation|SetWorldLocation _staticmesh (+ (Transformation|GetWorldLocation _staticmesh) "0, 0,1000.000000") false false)))))

(event EventBeginPlay
  (bind _staticmesh (Variables|Default|GetStaticMesh))
  (Transformation|SetWorldLocation _staticmesh (+ (Transformation|GetWorldLocation _staticmesh) "0, 0,-1000.000000") false false)
  (Rendering|SetVisibility _staticmesh false false))

(fn ConstructionScript)