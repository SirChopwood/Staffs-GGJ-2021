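; Placeable hiding spot that shows a configurable mesh and reveals a hidden bomb when RevealBomb is called.
; The construction script applies the mesh and reveal particle, moving the Niagara component to the configured bomb offset, raised slightly in world Z.
; RevealBomb uses that component as the spawn marker, removing the raise to spawn the bomb type with a wires defusal widget.
; It then plays the effect and sets a flag so it runs only once.
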(fn ConstructionScript
  (bind _niagara (Variables|Default|GetNiagara))
  (Transformation|AddLocalOffset _niagara (Variables|Default|GetRevealed%20Bomb%20Location) false false)
  (Transformation|AddWorldOffset _niagara "0, 0,100.000000" false false)
  (Class|NiagaraComponent|SetAsset _niagara (Variables|Default|GetReveal%20Particle))
  (Components|StaticMesh|SetStaticMesh (Variables|Default|GetStaticMesh) (Variables|Default|GetLocation%20Mesh)))

(fn RevealBomb
  (if (not (Variables|Default|GetRevealed))
    (Game|SpawnActorfromClass (Variables|Default|GetHidden%20Bomb%20Type) (Math|Transform|MakeTransform (- (Transformation|GetWorldLocation (Variables|Default|GetNiagara)) "0, 0,100.000000") "0,180.000000, 0" "1,1,1") "AdjustIfPossibleButAlwaysSpawn" 0 "/Game/Blueprints/DefusalWidget_Wires.DefusalWidget_Wires_C" 0)
    (Components|Activation|Activate (Variables|Default|GetNiagara) false)
    (Variables|Default|SetRevealed true)))