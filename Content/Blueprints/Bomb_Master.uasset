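; Base bomb Blueprint with a countdown display that can be defused or explode.
; A looping half-second timer drives a FlipFlop, counting down once per second while armed and blinking the text during the final 15 seconds.
; Explode opens the player's fail screen and activates Niagara particles, while Defuse stops the timer and shows a green "SAFE".
; The construction script applies the configurable bomb material.
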(event Custom|FuseTimer
  (Utilities|FlowControl|FlipFlop
    (:A
      (if (Variables|Default|GetArmed)
        (if (<= (Variables|Default|GetSeconds%20Remaining) 0.0)
          (CallFunction|Explode)
          (Utilities|Time|ClearandInvalidateTimerbyHandle (Variables|Default|GetFuseTimerRef))
          (else
            (bind _output_get (Variables|Default|SetSeconds%20Remaining (- (Variables|Default|GetSeconds%20Remaining) 1.0)))
            (Rendering|Components|TextRender|SetText (Variables|Default|GetTextRender) (Utilities|Text|ToText(Float) _output_get "HalfToEven" false true 3 3 0 0))
            (Rendering|SetVisibility (Variables|Default|GetTextRender) true false)))))
    (:B
      (if (<= (Variables|Default|GetSeconds%20Remaining) 15.0)
        (Rendering|SetVisibility (Variables|Default|GetTextRender) false false)))))

(event EventBeginPlay
  (bind _returnvalue (Utilities|Time|SetTimerbyEvent (delegate Custom|FuseTimer) 0.5 true))
  (Variables|Default|SetFuseTimerRef _returnvalue))

(fn ConstructionScript
  (Rendering|Material|SetMaterial (Variables|Default|GetBombMesh) 0 (Variables|Default|GetBombMaterial)))

(fn Defuse
  (bind _textrender (Variables|Default|GetTextRender))
  (Variables|Default|SetDefused true)
  (Variables|Default|SetArmed false)
  (Rendering|Components|TextRender|SetText _textrender (Utilities|Text|ToText(String) "SAFE"))
  (Rendering|Components|TextRender|SetTextRenderColor _textrender (Math|Color|MakeColor 100 255 100 255))
  (Rendering|SetVisibility _textrender true false)
  (Utilities|Time|ClearandInvalidateTimerbyHandle (Variables|Default|GetFuseTimerRef)))

(fn Explode
  (bind _asthird_person_character (Utilities|Casting|CastToThirdPersonCharacter (Game|Player|GetPlayerPawn 0)))
  (Default|EnterMenu _asthird_person_character "/Game/Blueprints/UI_FailScreen.UI_FailScreen_C")
  (Components|Activation|Activate (Variables|Default|GetNiagaraParticles) false))