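; NextLevelVolume is a trigger volume that moves the player to the next level once every bomb objective is complete.
; When a ThirdPersonCharacter overlaps EndVolume, it checks that all Bomb_Master actors are defused and all HiddenBombLocation actors are revealed.
; If both checks pass, it plays the character's UI transition animation, then opens the level named in LevelTo when the animation finishes.
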(event OnComponentBeginOverlap(EndVolume)
  (params (OverlappedComponent :type Primitive%20Component%20Object%20Reference) (OtherActor :type Actor%20Object%20Reference) (OtherComp :type Primitive%20Component%20Object%20Reference) (OtherBodyIndex :type Integer) (bFromSweep :type Boolean) (SweepResult :type Hit%20Result%20Structure%20%28by%20ref%29))
  (bind _asthird_person_character (Utilities|Casting|CastToThirdPersonCharacter OtherActor))
  (Variables|Default|SetGoodToMove true)
  (bind _outactors (Actor|GetAllActorsOfClass "/Game/Blueprints/Bomb_Master.Bomb_Master_C"))
  (for _array_element _outactors
    (if (not (Variables|/Game/Blueprints/Bomb_Master.Bomb_Master_C|GetDefused _array_element))
      (Variables|Default|SetGoodToMove false)))
  (bind _outactors_2 (Actor|GetAllActorsOfClass "/Game/Blueprints/HiddenBombLocation.HiddenBombLocation_C"))
  (for _array_element_2 _outactors_2
    (if (not (Variables|/Game/Blueprints/HiddenBombLocation.HiddenBombLocation_C|GetRevealed _array_element_2))
      (Variables|Default|SetGoodToMove false)))
  (if (Variables|Default|GetGoodToMove)
    (|PlayAnimationTimeRange (Variables|/Game/Blueprints/ThirdPersonCharacter.ThirdPersonCharacter_C|GetTransitionWidget _asthird_person_character) (Variables|/Game/Blueprints/ScreenTransition.ScreenTransition_C|GetUI_TransitionAnimation (Variables|/Game/Blueprints/ThirdPersonCharacter.ThirdPersonCharacter_C|GetTransitionWidget _asthird_person_character)) 0.0 0.0 1 "Forward" 1.0
      (:Finished
        (Game|OpenLevel(byName) (Variables|Default|GetLevelTo))))))

(fn ConstructionScript)